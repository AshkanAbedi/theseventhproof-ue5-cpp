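; Master HUD that creates the base HUD widget and swaps the crosshair icon according to what the player looks at.
; BeginPlay sets game-only input, adds WP_BaseHUD to the viewport and caches the BP_PlayerCharacter.
; ChangeIcon matches the class of the character's ObjectLookingAt to select, pickup or read icons, applied to InteractionWidget's InteractIcon.
; SetDefault restores the plain crosshair on that widget, which this graph never assigns.
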(event EventBeginPlay
  (bind _returnvalue (Game|Player|GetOwningPlayerController))
  ;[1 1 1] Initializing HUD
  (Input|SetInputModeGameOnly _returnvalue false)
  (bind _returnvalue_2 (UserInterface|CreateWidget "/Game/Dynamic/Blueprints/Prototype/UserInterface/HUD/WP_BaseHUD.WP_BaseHUD_C" _returnvalue))
  (UserInterface|Viewport|AddtoViewport _returnvalue_2 0)
  (bind _asbp_player_character (Utilities|Casting|CastToBP_PlayerCharacter (Game|GetPlayerCharacter 0)))
  (Variables|Default|SetPlayerCharacter _asbp_player_character))

(event EventSetDefault
  ;[1 1 1] Changing Crosshair Icon Based on Different Situations
  (Appearance|SetBrushfromTexture (Variables|/Game/Static/UI/Test/HUD/Widgets/InteractionWidget.InteractionWidget_C|GetInteractIcon (Variables|Default|GetInteractionWidget)) "/Game/Static/UI/Test/HUD/Textures/Crosshair.Crosshair" false))

(event EventChangeIcon
  ;[1 1 1] Changing Crosshair Icon Based on Different Situations
  (CallFunction|FindingCorrectIcon))

(fn ConstructionScript)

(fn FindingCorrectIcon
  (bind _interacticonlist (Variables|Default|GetInteractIconList))
  (bind _classnames (Variables|Default|GetClassNames))
  (bind _playercharacter (Variables|Default|GetPlayerCharacter))
  (bind (_pickup _inspect _read _select) (Utilities|Struct|BreakSTR_InteractIcons _interacticonlist))
  (bind (_bp_mi_switches _bp_mi_doors _bp_mi_drawers _bp_mi_keys _bp_mi_readables _bp_mi_interactonly) (Utilities|Struct|BreakSTR_ClassNames _classnames))
  (bind _objectlookingat (Variables|/Game/Dynamic/Blueprints/Test/PlayerCharacter/BP_PlayerCharacter.BP_PlayerCharacter_C|GetObjectLookingAt _playercharacter))
  (bind _returnvalue (Utilities|GetClass _objectlookingat))
  (switch int (Utilities|Array|FindItem (Utilities|Array|MakeArray (== _returnvalue _bp_mi_switches) (== _returnvalue _bp_mi_doors) (== _returnvalue _bp_mi_drawers) (== _returnvalue _bp_mi_keys) (== _returnvalue _bp_mi_readables) (== _returnvalue _bp_mi_interactonly)) true)
    (:0
      (Variables|Default|SetCurrentInteractIcon _select))
    (:1
      (Variables|Default|SetCurrentInteractIcon _select))
    (:2
      (Variables|Default|SetCurrentInteractIcon _select))
    (:3
      (Variables|Default|SetCurrentInteractIcon _pickup))
    (:4
      (Variables|Default|SetCurrentInteractIcon _read))
    (:5
      (Variables|Default|SetCurrentInteractIcon _select)))
  (Appearance|SetBrushfromTexture (Variables|/Game/Static/UI/Test/HUD/Widgets/InteractionWidget.InteractionWidget_C|GetInteractIcon (Variables|Default|GetInteractionWidget)) (Variables|Default|GetCurrentInteractIcon) false))