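; Master controller for the first-person player, turning Enhanced Input actions into move, look, run and crouch on the character.
; BeginPlay caches the HUD and character; InterfaceEnable blocks new actions, while run and crouch releases still apply.
; Running, blocked while crouched, raises walk speed and uses a reversible timeline to narrow FOV and ramp a post-process effect.
; Crouching pairs the Character crouch with a timeline that smoothly shifts camera height.
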(event Input|EnhancedActionEvents|EnhancedInputActionIA_Crouch
  (params (ActionValue :type Boolean) (ElapsedSeconds :type Float%20%28double-precision%29) (TriggeredSeconds :type Float%20%28double-precision%29) (InputAction :type Input%20Action%20Object%20Reference :default "/Game/Dynamic/Blueprints/Test/EnhancedInput/IA_Crouch.IA_Crouch"))
  (:Started
    (if (not (Variables|Default|GetInterfaceEnable))
      (Character|Crouch :!label _label)))
  (:Completed
    (goto _label Un%20Crouch)))

(event Input|EnhancedActionEvents|EnhancedInputActionIA_Move
  (params (ActionValue :type Vector%202D%20Structure) (ElapsedSeconds :type Float%20%28double-precision%29) (TriggeredSeconds :type Float%20%28double-precision%29) (InputAction :type Input%20Action%20Object%20Reference :default "/Game/Dynamic/Blueprints/Test/EnhancedInput/IA_Move.IA_Move"))
  (:Triggered
    (if (not (Variables|Default|GetInterfaceEnable))
      (CallFunction|Movement (.x ActionValue) (.y ActionValue)))))

(event Input|EnhancedActionEvents|EnhancedInputActionIA_Look
  (params (ActionValue :type Vector%202D%20Structure) (ElapsedSeconds :type Float%20%28double-precision%29) (TriggeredSeconds :type Float%20%28double-precision%29) (InputAction :type Input%20Action%20Object%20Reference :default "/Game/Dynamic/Blueprints/Test/EnhancedInput/IA_Look.IA_Look"))
  (:Triggered
    (if (not (Variables|Default|GetInterfaceEnable))
      (CallFunction|LookAround (.x ActionValue) (.y ActionValue)))))

(event Input|EnhancedActionEvents|EnhancedInputActionIA_Run
  (params (ActionValue :type Boolean) (ElapsedSeconds :type Float%20%28double-precision%29) (TriggeredSeconds :type Float%20%28double-precision%29) (InputAction :type Input%20Action%20Object%20Reference :default "/Game/Dynamic/Blueprints/Test/EnhancedInput/IA_Run.IA_Run"))
  (:Triggered
    (if (not (Variables|Default|GetInterfaceEnable))
      (|Run :!label _label)))
  (:Completed
    (goto _label Stop)))

(event EventBeginPlay
  (bind _asbp_master_hud (Utilities|CasttoValidHUD 1e+01)
    (:Success
      (Variables|Default|SetMasterHUD _asbp_master_hud)
      (bind _as_bp_player_character (Utilities|CasttoValidCharacter 0.0)
        (:Success
          (Variables|Default|SetPlayerCharacter _as_bp_player_character))))))

(fn ConstructionScript)

(fn Movement
  (params (RAxis%20Value :type Float%20%28double-precision%29) (FAxis%20Value :type Float%20%28double-precision%29))
  (bind _returnvalue (Game|GetPlayerCharacter 0))
  (bind _returnvalue_2 (Game|GetPlayerCharacter 0))
  (Pawn|Input|AddMovementInput _returnvalue (Transformation|GetActorRightVector _returnvalue) RAxis%20Value false)
  (Pawn|Input|AddMovementInput _returnvalue_2 (Transformation|GetActorForwardVector _returnvalue_2) FAxis%20Value false))

(fn LookAround
  (params (Yaw%20Value :type Float%20%28double-precision%29) (Pitch%20Value :type Float%20%28double-precision%29))
  (bind _returnvalue (Game|GetPlayerCharacter 0))
  (Pawn|Input|AddControllerPitchInput _returnvalue Pitch%20Value)
  (Pawn|Input|AddControllerYawInput _returnvalue (* Yaw%20Value -1.0)))