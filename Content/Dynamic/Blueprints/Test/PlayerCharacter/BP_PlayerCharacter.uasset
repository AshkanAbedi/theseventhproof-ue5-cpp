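; First-person player character that handles interaction, item inspection, a flashlight, an inventory widget toggle and an Attention focus effect.
; A looping timer line-traces from the camera to update the HUD icon and the looked-at actor through interfaces, feeding interact and inspect inputs.
; Inspection moves the item before the camera for look-driven rotation with adjusted focal distance.
; Attention uses a timeline to narrow FOV, desaturate and add vignette unless running.
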(event Custom|InitializeTracingTimer
  ;[1 1 1] Tracing
  (Utilities|Time|SetTimerbyEvent (delegate Custom|CheckTracing) 0.25 true))

(event Custom|CheckTracing
  ;[1 1 1] Tracing
  (CallFunction|Tracing))

(event Input|EnhancedActionEvents|EnhancedInputActionIA_Inspect
  (params (ActionValue :type Boolean) (ElapsedSeconds :type Float%20%28double-precision%29) (TriggeredSeconds :type Float%20%28double-precision%29) (InputAction :type Input%20Action%20Object%20Reference :default "/Game/Dynamic/Blueprints/Test/EnhancedInput/IA_Inspect.IA_Inspect"))
  ;[1 1 1] Inspection
  (:Triggered
    (Utilities|FlowControl|FlipFlop
      (:A
        (CallFunction|InspectInterface))
      (:B
        (CallFunction|ReturnfromInspect)))))

(event Input|EnhancedActionEvents|EnhancedInputActionIA_Inventory
  (params (ActionValue :type Boolean) (ElapsedSeconds :type Float%20%28double-precision%29) (TriggeredSeconds :type Float%20%28double-precision%29) (InputAction :type Input%20Action%20Object%20Reference :default "/Game/Dynamic/Blueprints/Test/EnhancedInput/IA_Inventory.IA_Inventory"))
  (bind _inventorywidget (Variables|Inventory|GetInventoryWidget))
  ;[1 1 1] Debug Inventory
  (:Started
    (Utilities|FlowControl|FlipFlop
      (:A
        (UserInterface|Viewport|AddtoViewport _inventorywidget 0))
      (:B
        (Widget|RemovefromParent _inventorywidget)))))

(event Input|EnhancedActionEvents|EnhancedInputActionIA_Look
  (params (ActionValue :type Vector%202D%20Structure) (ElapsedSeconds :type Float%20%28double-precision%29) (TriggeredSeconds :type Float%20%28double-precision%29) (InputAction :type Input%20Action%20Object%20Reference :default "/Game/Dynamic/Blueprints/Test/EnhancedInput/IA_Look.IA_Look"))
  ;[1 1 1] Inspection
  (:Triggered
    (CallFunction|RotateItem (.x ActionValue) (.y ActionValue))))

(event Input|EnhancedActionEvents|EnhancedInputActionIA_Flashlight
  (params (ActionValue :type Boolean) (ElapsedSeconds :type Float%20%28double-precision%29) (TriggeredSeconds :type Float%20%28double-precision%29) (InputAction :type Input%20Action%20Object%20Reference :default "/Game/Dynamic/Blueprints/Prototype/EnhancedInput/IA_Flashlight.IA_Flashlight"))
  ;[1 1 1] Flashlight
  (:Started
    (Utilities|TriggerFlashlight)))

(event Input|EnhancedActionEvents|EnhancedInputActionIA_Interact
  (params (ActionValue :type Boolean) (ElapsedSeconds :type Float%20%28double-precision%29) (TriggeredSeconds :type Float%20%28double-precision%29) (InputAction :type Input%20Action%20Object%20Reference :default "/Game/Dynamic/Blueprints/Test/EnhancedInput/IA_Interact.IA_Interact"))
  ;[1 1 1] Interact
  (:Triggered
    (CallFunction|Interaction)))

(event EventBeginPlay
  ;[1 1 1] BeginPlayEvents
  (CallFunction|BeginPlayEvents))

(fn ConstructionScript)

(fn Tracing
  (bind _playercontroller (Variables|Controller|GetPlayerController))
  (bind _fpscamera (Variables|Default|GetFpsCamera))
  (bind _returnvalue (Transformation|GetWorldLocation _fpscamera))
  (bind _masterhud (Variables|/Game/Dynamic/Blueprints/Test/GameMode/BP_MasterController.BP_MasterController_C|GetMasterHUD _playercontroller))
  (bind _outhit (Collision|LineTraceByChannel _returnvalue (+ _returnvalue (* (Math|Vector|GetForwardVector _fpscamera) (Variables|ObjectInteraction|GetDistanceFromObject))) "TraceTypeQuery1" false 0 "None"))
  (bind _output_get (Variables|ObjectInteraction|SetObjectLookingAt (.HitActor (Collision|BreakHitResult _outhit))))
  (if (Utilities|DoesObjectImplementInterface _output_get "/Game/Dynamic/Blueprints/Test/GameLogic/BPI_HandleInteractIcon.BPI_HandleInteractIcon_C")
    (Default|ChangeIcon _masterhud)
    (if (Utilities|DoesObjectImplementInterface _output_get "/Game/Dynamic/Blueprints/Test/GameLogic/BPI_InspectInterface.BPI_InspectInterface_C")
      (Class|BPIInspectInterface|InspectInterface(Message) (Variables|ObjectInteraction|GetObjectLookingAt)))
    (else
      (Default|SetDefault _masterhud)
      (Variables|ObjectInspection|SetInspectionKeyEnable false))))

(fn EnhancedInput
  (bind _asplayer_controller (Utilities|Casting|CastToPlayerController (Pawn|GetController)))
  (Utilities|IsValid (PlayerController|LocalPlayerSubsystems|GetEnhancedInputLocalPlayerSubsystem _asplayer_controller)
    (:Is%20Valid
      (Input|AddMappingContext (PlayerController|LocalPlayerSubsystems|GetEnhancedInputLocalPlayerSubsystem _asplayer_controller) "/Game/Dynamic/Blueprints/Test/EnhancedInput/IM_Context.IM_Context" 0 "(bIgnoreAllPressedKeysUntilRelease=True,bForceImmediately=False)"))))

(fn Interaction
  (if (not (Variables|/Game/Dynamic/Blueprints/Test/GameMode/BP_MasterController.BP_MasterController_C|GetInterfaceEnable (Variables|Controller|GetPlayerController)))
    (Class|BPIInteractInterface|Interact(Message) (Variables|ObjectInteraction|GetObjectLookingAt))))

(fn BeginPlayEvents
  (bind _asbp_master_controller (Utilities|Casting|CastToBP_MasterController (Game|GetPlayerController 0)))
  (Variables|Controller|SetPlayerController _asbp_master_controller)
  (CallFunction|InitializeTracingTimer)
  (CallFunction|EnhancedInput)
  (bind _returnvalue (UserInterface|CreateWidget "/Game/Static/UI/Test/HUD/Widgets/InventoryWidget02.InventoryWidget02_C"))
  (Variables|Inventory|SetInventoryWidget _returnvalue))

(fn DebugInventory
  (for _array_element (Variables|Inventory|GetMainInventory)
    (Development|PrintString (Utilities|GetDisplayName _array_element))))

(fn InspectInterface
  (bind _returnvalue (Game|GetPlayerCameraManager 0))
  (bind _playercontroller (Variables|Controller|GetPlayerController))
  (if (Variables|ObjectInspection|GetInspectionKeyEnable)
    (Class|BPIInspectInterface|Inspection(Message) (Variables|ObjectInteraction|GetObjectLookingAt))
    (Variables|ObjectInspection|SetRotationKeysEnable true)
    (Variables|/Game/Dynamic/Blueprints/Test/GameMode/BP_MasterController.BP_MasterController_C|SetInterfaceEnable _playercontroller true)
    (Widget|RemovefromParent (Variables|/Game/Dynamic/Blueprints/Test/GameMode/BP_MasterHUD.BP_MasterHUD_C|GetInteractionWidget (Variables|/Game/Dynamic/Blueprints/Test/GameMode/BP_MasterController.BP_MasterController_C|GetMasterHUD _playercontroller)))
    (Transformation|SetWorldLocation (Variables|Default|GetInspectableItem) (+ (Camera|GetCameraLocation _returnvalue) (* (Math|Vector|GetForwardVector (Camera|GetCameraRotation _returnvalue)) (Variables|ObjectInspection|GetItemDistanceToCamera))) false false)
    (Variables|/Script/Engine.CameraComponent|SetPostProcessSettings (Variables|Default|GetFpsCamera) (Utilities|Struct|MakePostProcessSettings 24.576 1.0 2e+01))
    (Variables|ObjectInspection|SetIsInspecting true)))

(fn ReturnfromInspect
  (Class|BPIInspectInterface|CancelInspectInterface(Message) (Variables|ObjectInteraction|GetObjectLookingAt))
  (Variables|/Script/Engine.CharacterMovementComponent|SetMaxWalkSpeed (Variables|Character|GetCharacterMovement) 1.5e+02)
  (Variables|ObjectInspection|SetRotationKeysEnable false)
  (Variables|/Game/Dynamic/Blueprints/Test/GameMode/BP_MasterController.BP_MasterController_C|SetInterfaceEnable (Variables|Controller|GetPlayerController) false)
  (UserInterface|Viewport|AddtoViewport (Variables|/Game/Dynamic/Blueprints/Test/GameMode/BP_MasterHUD.BP_MasterHUD_C|GetInteractionWidget (Variables|/Game/Dynamic/Blueprints/Test/GameMode/BP_MasterController.BP_MasterController_C|GetMasterHUD (Variables|Controller|GetPlayerController))) 0)
  (Variables|/Script/Engine.CameraComponent|SetPostProcessSettings (Variables|Default|GetFpsCamera) (Utilities|Struct|MakePostProcessSettings 24.576))
  (Variables|ObjectInspection|SetIsInspecting false))

(fn RotateItem
  (params (Value01 :type Float%20%28double-precision%29) (Value02 :type Float%20%28double-precision%29))
  (if (Variables|ObjectInspection|GetRotationKeysEnable)
    (Transformation|AddWorldRotation (Variables|Default|GetInspectableItem) (Math|Rotator|MakeRotator (* Value01 (Variables|ObjectInspection|GetRotationItemSpeed)) 0.0 (* Value02 (Variables|ObjectInspection|GetRotationItemSpeed))) false false)))

(fn ChangeIcon)

(event Input|EnhancedActionEvents|EnhancedInputActionIA_Attention
  (params (ActionValue :type Boolean) (ElapsedSeconds :type Float%20%28double-precision%29) (TriggeredSeconds :type Float%20%28double-precision%29) (InputAction :type Input%20Action%20Object%20Reference :default "/Game/Dynamic/Blueprints/Test/EnhancedInput/IA_Attention.IA_Attention"))
  (bind _fpscamera (Variables|Default|GetFpsCamera))
  (:Triggered
    (if (not (Variables|/Game/Dynamic/Blueprints/Test/GameMode/BP_MasterController.BP_MasterController_C|GetIsRunning (Variables|Controller|GetPlayerController)))
      (bind _lerpvalue (Timeline|Lerp Play)
        (:Update
          (Camera|SetFieldOfView _fpscamera (Math|Float|Lerp 9e+01 5e+01 _lerpvalue))
          (Utilities|Struct|SetmembersinPostProcessSettings (Variables|/Script/Engine.CameraComponent|GetPostProcessSettings _fpscamera) (Math|Vector4|MakeVector4 (Math|Float|Lerp 1.0 0.0 _lerpvalue) (Math|Float|Lerp 1.0 0.0 _lerpvalue) (Math|Float|Lerp 1.0 0.0 _lerpvalue) (Math|Float|Lerp 1.0 0.0 _lerpvalue)) (Math|Float|Lerp 0.0 12.0 _lerpvalue) (Math|Float|Lerp 0.0 0.8 _lerpvalue))))))
  (:Completed
    (Timeline|Lerp Reverse)))