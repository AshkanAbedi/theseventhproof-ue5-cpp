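; BP_MI_Switches is an interactable light switch that turns a light on and off.
; Its Interact event calls LightSwitch, which branches on the LightOn flag to toggle the visibility of Light01 and update the flag.
; Each direction plays its own sound at the actor's location, and the construction script only calls the parent's.
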(event EventInteract
  (CallFunction|LightSwitch))

(fn ConstructionScript
  (|CallParentFunction))

(fn LightSwitch
  (bind _light01 (Variables|Default|GetLight01))
  (if (Variables|GeneralSetting|GetLightOn)
    (Audio|PlaySoundatLocation (Variables|Default|GetFirstSound) (Transformation|GetActorLocation) "0, 0, 0" 1.0 1.0 0.0 0 0 0 0)
    (Rendering|SetVisibility _light01 false false)
    (Variables|GeneralSetting|SetLightOn false)
    (else
      (Audio|PlaySoundatLocation (Variables|Default|GetSecondSound) (Transformation|GetActorLocation) "0, 0, 0" 1.0 1.0 0.0 0 0 0 0)
      (Rendering|SetVisibility _light01 true false)
      (Variables|GeneralSetting|SetLightOn true))))