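; Pickup item actor that the player collects into the main inventory through an Interact event.
; ItemPickup adds the actor's own reference to BP_PlayerCharacter's MainInventory without duplicates, calls a sound at its location, then destroys the actor.
; It then loops over the inventory, printing each item's name and, on every iteration, pushing the music sound mix and playing the clue music cue.
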(event EventInteract
  (CallFunction|ItemPickup))

(fn ConstructionScript
  (|CallParentFunction))

(fn ItemPickup
  (bind _asbp_player_character (Utilities|Casting|CastToBP_PlayerCharacter (Game|GetPlayerCharacter 0)))
  (Utilities|Array|AddUnique (Variables|/Game/Dynamic/Blueprints/Test/PlayerCharacter/BP_PlayerCharacter.BP_PlayerCharacter_C|GetMainInventory _asbp_player_character) self)
  (Audio|PlaySoundatLocation 0 (Transformation|GetActorLocation) "0, 0, 0" 1.0 1.0 0.0 0 0 0 0)
  (Actor|DestroyActor)
  (for _array_element (Variables|/Game/Dynamic/Blueprints/Test/PlayerCharacter/BP_PlayerCharacter.BP_PlayerCharacter_C|GetMainInventory _asbp_player_character)
    (Development|PrintString (Utilities|GetDisplayName _array_element))
    (Audio|PushSoundMixModifier "/Game/Static/Audio/Classes/SMix_Music.SMix_Music")
    (Audio|PlaySound2D "/Game/Static/Audio/InProject/SW_MU_Clue01_Cue.SW_MU_Clue01_Cue" 1.0 1.0 0.0 0 0)))