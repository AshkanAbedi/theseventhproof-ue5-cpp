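; Interactable door that swings open and closed, optionally locked behind a key item.
; On Interact, a valid RequiredKey must be in the player character's MainInventory, otherwise a locked message prints and a sound plays.
; OpenClose uses a FlipFlop to play or reverse a timeline that lerps MainObject's yaw between two rotations, with a sound for each direction.
; An IsOpening flag ignores input while the door moves.
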(event EventInteract
  (Utilities|IsValid (Variables|GeneralSettings|GetRequiredKey)
    (:Is%20Valid
      (bind _returnvalue (CallFunction|CheckKey))
      (if _returnvalue
        (|Open/Close :!label _label)
        (else
          (CallFunction|Locked))))
    (:Is%20Not%20Valid
      (goto _label))))

(fn ConstructionScript
  (|CallParentFunction))

(fn Locked
  (Development|PrintString "THE DOOR IS LOCKED")
  (Audio|PlaySoundatLocation (Variables|Sounds|GetLockedSound) (Transformation|GetActorLocation) "0, 0, 0" 1.0 1.0 0.0 0 0 0 0))

(fn CheckKey
  (bind _asbp_player_character (Utilities|Casting|CastToBP_PlayerCharacter (Game|GetPlayerCharacter 0)))
  (return (Utilities|Array|ContainsItem (Variables|/Game/Dynamic/Blueprints/Test/PlayerCharacter/BP_PlayerCharacter.BP_PlayerCharacter_C|GetMainInventory _asbp_player_character) (Variables|GeneralSettings|GetRequiredKey))))