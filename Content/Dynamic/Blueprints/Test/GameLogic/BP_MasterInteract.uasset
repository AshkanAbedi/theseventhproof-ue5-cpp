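; BP_MasterInteract is an interactable object that the player can inspect, driven by three events for checking, starting and cancelling inspection.
; If flagged inspectable, it caches the player character and enables its inspection key.
; Inspection copies MainObject's mesh onto the player's InspectableItem component, showing that and hiding the world object.
; Cancelling clears the player's mesh, hides it and restores MainObject's visibility.
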(event EventCancelInspectInterface
  (CallFunction|CancelInspection))

(event EventInspectInterface
  (params (PlayerCharacter :type BP%20Player%20Character%20Object%20Reference))
  (CallFunction|CheckInspectable))

(event EventInspection
  (CallFunction|InitializeInspection))

(fn ConstructionScript)

(fn CheckInspectable
  (if (Variables|Inspection|GetInspectableItem)
    (bind _asbp_player_character (Utilities|Casting|CastToBP_PlayerCharacter (Game|GetPlayerCharacter 0)))
    (bind _output_get (Variables|Default|SetPlayerCharacter _asbp_player_character))
    (Variables|/Game/Dynamic/Blueprints/Test/PlayerCharacter/BP_PlayerCharacter.BP_PlayerCharacter_C|SetInspectionKeyEnable _output_get true)))

(fn InitializeInspection
  (bind _mainobject (Variables|Components|GetMainObject))
  (bind _playercharacter (Variables|Default|GetPlayerCharacter))
  (bind _inspectableitem (Variables|/Game/Dynamic/Blueprints/Test/PlayerCharacter/BP_PlayerCharacter.BP_PlayerCharacter_C|GetInspectableItem _playercharacter))
  (if (Utilities|IsValid _playercharacter)
    (Components|StaticMesh|SetStaticMesh _inspectableitem (Variables|/Script/Engine.StaticMeshComponent|GetStaticMesh _mainobject))
    (Rendering|SetVisibility _inspectableitem true false)
    (Rendering|SetVisibility _mainobject false false)))

(fn CancelInspection
  (bind _playercharacter (Variables|Default|GetPlayerCharacter))
  (bind _inspectableitem (Variables|/Game/Dynamic/Blueprints/Test/PlayerCharacter/BP_PlayerCharacter.BP_PlayerCharacter_C|GetInspectableItem _playercharacter))
  (if (Utilities|IsValid _playercharacter)
    (Components|StaticMesh|SetStaticMesh _inspectableitem 0)
    (Rendering|SetVisibility _inspectableitem false false)
    (Rendering|SetVisibility (Variables|Components|GetMainObject) true false)))