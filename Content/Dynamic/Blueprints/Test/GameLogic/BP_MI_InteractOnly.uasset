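; Interactable test Blueprint that shows a text prompt with a voice line when interacted with.
; BeginPlay creates and stores the prompt widget.
; Interact passes the text, reading time and voice to ObjectPrompt, which uses a DoOnce gate to set the text, add the widget to the viewport and play the 2D sound.
; The widget is removed after the reading time, followed by a short delay.
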(event EventInteract
  (Utilities|ObjectPrompt (Variables|Content|GetPromptText) (Variables|Content|GetReadingTime) (Variables|Default|GetVoice)))

(event EventBeginPlay
  (bind _returnvalue (UserInterface|CreateWidget "/Game/Static/UI/Test/HUD/Widgets/PromptWidget.PromptWidget_C"))
  (Variables|Default|SetPromptWidget _returnvalue))

(fn ConstructionScript
  (|CallParentFunction))