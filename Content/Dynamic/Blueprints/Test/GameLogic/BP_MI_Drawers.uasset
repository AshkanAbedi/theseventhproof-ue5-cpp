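; Interactable drawer that slides open and closed, optionally locked behind a key item in the player's inventory.
; Interact checks RequiredKey, then either runs the Open/Close macro or plays locked feedback.
; The macro's FlipFlop plays or reverses a Timeline that lerps the mesh's X position, with an IsOpening guard against re-triggering.
; Helpers to spawn and attach an item or readable inside exist but are not wired to run.
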(event EventBeginPlay)

(event EventInteract
  (Utilities|IsValid (Variables|GeneralSettings|GetRequiredKey)
    (:Is%20Valid
      (bind _returnvalue (CallFunction|CheckKey))
      (if _returnvalue
        (|Open/Close :!label _label)
        (else
          (CallFunction|Locked))))
    (:Is%20Not%20Valid
      (goto _label))))

(fn ConstructionScript
  (|CallParentFunction))

(fn Locked
  (Development|PrintString "PLAY MONOLOGUE \"THE DOOR IS LOCKED\"")
  (Audio|PlaySoundatLocation (Variables|Sounds|GetLockedSound) (Transformation|GetActorLocation) "0, 0, 0" 1.0 1.0 0.0 0 0 0 0))

(fn CheckKey
  (bind _asbp_player_character (Utilities|Casting|CastToBP_PlayerCharacter (Game|GetPlayerCharacter 0)))
  (return (Utilities|Array|ContainsItem (Variables|/Game/Dynamic/Blueprints/Test/PlayerCharacter/BP_PlayerCharacter.BP_PlayerCharacter_C|GetMainInventory _asbp_player_character) (Variables|GeneralSettings|GetRequiredKey))))

(fn AddInsideReadableItem
  (bind _returnvalue (Game|SpawnActorfromClass "/Game/Dynamic/Blueprints/Test/GameLogic/BP_MI_Readables.BP_MI_Readables_C" (Transformation|GetActorTransform) "Undefined" 0 0))
  (bind _output_get (Variables|InsideDocument|SetBPReadable _returnvalue))
  (Variables|/Game/Dynamic/Blueprints/Test/GameLogic/BP_MasterInteract.BP_MasterInteract_C|SetInspectableItem _output_get (Variables|InsideDocument|GetCanInspectDoc))
  (Components|StaticMesh|SetStaticMesh (Variables|/Game/Dynamic/Blueprints/Test/GameLogic/BP_MasterInteract.BP_MasterInteract_C|GetMainObject _returnvalue) (Variables|InsideDocument|GetInsideReadableMesh))
  (Transformation|AttachComponentToComponent _returnvalue (Variables|Default|GetMainObject) "None" "KeepWorld" "KeepWorld" "KeepRelative" true)
  (Class|SceneComponent|AddLocalTransform (Variables|/Game/Dynamic/Blueprints/Test/GameLogic/BP_MasterInteract.BP_MasterInteract_C|GetMainObject _returnvalue) (Variables|InsideDocument|GetInsideReadableTransform) false false)
  (Variables|/Game/Dynamic/Blueprints/Test/GameLogic/BP_MI_Readables.BP_MI_Readables_C|SetContent _returnvalue (Variables|InsideDocument|GetReadableContent)))

(fn AddInsideItem
  (bind _returnvalue (Game|SpawnActorfromClass "/Game/Dynamic/Blueprints/Test/GameLogic/BP_MI_Items.BP_MI_Items_C" (Transformation|GetActorTransform) "Undefined" 0 0))
  (bind _output_get (Variables|InsideItem|SetBPItem _returnvalue))
  (Variables|/Game/Dynamic/Blueprints/Test/GameLogic/BP_MasterInteract.BP_MasterInteract_C|SetInspectableItem _output_get (Variables|InsideItem|GetCanInspectItem))
  (Components|StaticMesh|SetStaticMesh (Variables|/Game/Dynamic/Blueprints/Test/GameLogic/BP_MasterInteract.BP_MasterInteract_C|GetMainObject _output_get) (Variables|InsideItem|GetInsideItemMesh))
  (Transformation|AttachComponentToComponent _output_get (Variables|Default|GetMainObject) "None" "KeepWorld" "KeepWorld" "KeepRelative" true)
  (Class|SceneComponent|AddLocalTransform (Variables|/Game/Dynamic/Blueprints/Test/GameLogic/BP_MasterInteract.BP_MasterInteract_C|GetMainObject _output_get) (Variables|InsideItem|GetInsideItemTransform) false false))