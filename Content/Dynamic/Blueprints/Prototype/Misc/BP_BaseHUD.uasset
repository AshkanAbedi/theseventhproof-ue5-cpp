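; Prototype HUD that handles crosshair, prompt and reading feedback for player interactions.
; On BeginPlay it creates the HUD and inventory widgets, adds only the HUD to the viewport, and binds to BP_BasePlayer delegates.
; The object class's index in ClassArray selects the crosshair icon and interaction response.
; Observables and locked doors show timed prompt text, while readables show an image over background blur until cancel clears it and restores Normal player state.
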(event Custom|OnSeeingInteractable_Event
  (params (InteractableType :type Object%20Class%20Reference))
  ;[1 1 1] Changing Crosshair Icon
  (bind _returnvalue (|CheckObjectClass))
  (if (Utilities|Enum|Equal(Enum) (Variables|/Script/TheSeventhProof.PlayerCharacter|GetPlayerStates (Variables|Default|GetBP_BasePlayer)) "EPS_Inspecting")
    (CallFunction|SelectCrosshair "/Game/ExternalPacks/EdithFinchRoom/Common/MasterMaterial/DefaultTextures/dot_alpha.dot_alpha" "(X=5.000000,Y=5.000000)" 0.0)
    (else
      (switch int _returnvalue
        (:0
          (CallFunction|SelectCrosshair "/Game/Static/UI/Test/HUD/Textures/view.view" "(X=40.000000,Y=40.000000)" 1.0))
        (:1
          (CallFunction|SelectCrosshair "/Game/Static/UI/Test/HUD/Textures/Open.Open" "(X=40.000000,Y=40.000000)" 1.0))
        (:2
          (CallFunction|SelectCrosshair "/Game/Static/UI/Test/HUD/Textures/Read.Read" "(X=40.000000,Y=40.000000)" 1.0))
        (:3
          (CallFunction|SelectCrosshair "/Game/Static/UI/Test/HUD/Textures/Inspect.Inspect" "(X=40.000000,Y=40.000000)" 1.0))
        (:4
          (CallFunction|SelectCrosshair "/Game/Static/UI/Test/HUD/Textures/Switch.Switch" "(X=40.000000,Y=40.000000)" 1.0))
        (:5
          (CallFunction|SelectCrosshair "/Game/Static/UI/Test/HUD/Textures/Pick.Pick" "(X=40.000000,Y=40.000000)" 1.0))))))

(event Custom|OnInteracting_Event
  (params (InteractedObject :type Actor%20Object%20Reference))
  (bind _wp_basehud (Variables|Default|GetWP_BaseHUD))
  (bind _prompttext (Variables|/Script/TheSeventhProof.BaseHUD|GetPromptText _wp_basehud))
  ;[1 0.849 0.396] Interacting with Objects
  (switch int (Utilities|Array|FindItem (Variables|Default|GetClassArray) (Utilities|GetClass InteractedObject))
    (:0
      ;[1 1 1] Observables
      (bind (_storydelay _prompttext_2) (CallFunction|InteractObservables InteractedObject))
      (Utilities|FlowControl|Delay _storydelay)
      (Variables|/Script/UMG.TextBlock|SetText _prompttext_2 ""))
    (:1
      ;[1 1 1] Locked Doors
      (bind _asbp_base_doors (Utilities|Casting|CastToBP_BaseDoors InteractedObject))
      (switch Utilities|FlowControl|Switch|SwitchonEDoorStates (Variables|/Script/TheSeventhProof.Doors|GetDoorState _asbp_base_doors)
        (:EDS_StateNormal
          (Variables|/Script/TheSeventhProof.Doors|SetLockMessage _asbp_base_doors "" :!label _label))
        (:EDS_StateLocked
          (Variables|/Script/UMG.TextBlock|SetText _prompttext (Variables|/Script/TheSeventhProof.Doors|GetLockMessage _asbp_base_doors))
          (Utilities|FlowControl|Delay (Variables|/Script/TheSeventhProof.Doors|GetMessageDuration _asbp_base_doors))
          (Variables|/Script/UMG.TextBlock|SetText _prompttext ""))
        (:EDS_StateUnlocking
          (goto _label))))
    (:2
      ;[1 1 1] Readings
      (CallFunction|InteractReading InteractedObject))))

(event Custom|OnInputCancel
  ;[1 1 1] Readings
  (CallFunction|CancelReading))

(event EventBeginPlay
  ;[1 1 1] Initialize HUD
  (bind _output_get (CallFunction|CreateWidgets))
  (EventDispatchers|AssignOnSeeingInteractable _output_get (delegate Custom|OnSeeingInteractable_Event))
  (EventDispatchers|BindEventtoOnInteracting _output_get (delegate Custom|OnInteracting_Event))
  (EventDispatchers|BindEventtoOnCancelInputDelegate _output_get (delegate Custom|OnInputCancel)))

(fn ConstructionScript)

(fn SelectCrosshair
  (params (Image :type Texture%202D%20Object%20Reference) (Size :type Vector%202D%20Structure :default "(X=40.000000,Y=40.000000)") (InOpacity :type Float%20%28single-precision%29))
  (bind _wp_basehud (Variables|Default|GetWP_BaseHUD))
  (bind _crosshairicons (Variables|/Script/TheSeventhProof.BaseHUD|GetCrosshairIcons _wp_basehud))
  (Appearance|SetBrushfromTexture _crosshairicons Image false)
  (Class|Image|SetDesiredSizeOverride _crosshairicons Size)
  (Class|Image|SetOpacity _crosshairicons InOpacity)
  (return))

(fn CreateWidgets
  (bind _returnvalue (Game|Player|GetOwningPlayerController))
  (Input|SetInputModeGameOnly _returnvalue false)
  (bind _returnvalue_2 (UserInterface|CreateWidget "/Game/Dynamic/Blueprints/Prototype/UserInterface/HUD/WP_BaseHUD.WP_BaseHUD_C" _returnvalue))
  (bind _output_get (Variables|Default|SetWP_BaseHUD _returnvalue_2))
  (UserInterface|Viewport|AddtoViewport _output_get 0)
  (bind _returnvalue_3 (UserInterface|CreateWidget "/Game/Dynamic/Blueprints/Prototype/UserInterface/Inventory/WP_BaseInventory.WP_BaseInventory_C" _returnvalue))
  (Variables|Default|SetWP_BaseInventory _returnvalue_3)
  (bind _asbp_base_player (Utilities|Casting|CastToBP_BasePlayer (Game|GetPlayerCharacter 0)))
  (bind _output_get_2 (Variables|Default|SetBP_BasePlayer _asbp_base_player))
  (return _output_get_2))

(fn InteractObservables
  (params (Cast :type Actor%20Object%20Reference))
  (bind _wp_basehud (Variables|Default|GetWP_BaseHUD))
  (bind _prompttext (Variables|/Script/TheSeventhProof.BaseHUD|GetPromptText _wp_basehud))
  (bind _asbp_base_observables (Utilities|Casting|CastToBP_BaseObservables Cast)
    (:then
      (Variables|/Script/UMG.TextBlock|SetText _prompttext (Variables|/Script/TheSeventhProof.Observables|GetStoryText _asbp_base_observables))
      (return (Variables|/Script/TheSeventhProof.Observables|GetStoryDelay _asbp_base_observables) _prompttext))
    (:CastFailed
      (return 0.0 0))))

(fn InteractDoors
  (params (Cast :type Object%20Object%20Reference))
  (bind _asbp_base_doors (Utilities|Casting|CastToBP_BaseDoors Cast)
    (:then
      (if true
        (return _asbp_base_doors)
        (else
          (Variables|/Script/UMG.TextBlock|SetText (Variables|/Script/TheSeventhProof.BaseHUD|GetPromptText (Variables|Default|GetWP_BaseHUD)) "CLEARING THE TEXT"))))
    (:CastFailed
      (return _asbp_base_doors))))

(fn InteractReading
  (params (Object :type Object%20Object%20Reference))
  (bind _wp_basehud (Variables|Default|GetWP_BaseHUD))
  (bind _asbp_base_reads (Utilities|Casting|CastToBP_BaseReads Object)
    (:then
      (Class|Image|SetBrush (Variables|/Game/Dynamic/Blueprints/Prototype/UserInterface/HUD/WP_BaseHUD.WP_BaseHUD_C|GetReadingImage _wp_basehud) (Utilities|Struct|MakeSlateBrush "Image" "NoTile" "NoMirror" "(X=700.000000,Y=900.000000)" "(Left=0.000000,Top=0.000000,Right=0.000000,Bottom=0.000000)" "(SpecifiedColor=(R=1.000000,G=1.000000,B=1.000000,A=1.000000),ColorUseRule=UseColor_Specified)" "(CornerRadii=(X=0.000000,Y=0.000000,Z=0.000000,W=1.000000),Color=(SpecifiedColor=(R=0.000000,G=0.000000,B=0.000000,A=0.000000),ColorUseRule=UseColor_Specified),Width=0.000000,RoundingType=HalfHeightRadius,bUseBrushTransparency=False)" (Variables|/Script/TheSeventhProof.Reads|GetReadImage _asbp_base_reads)))
      (Class|BackgroundBlur|SetBlurStrength (Variables|/Game/Dynamic/Blueprints/Prototype/UserInterface/HUD/WP_BaseHUD.WP_BaseHUD_C|GetBackgroundBlur _wp_basehud) 5.0))
    (:CastFailed
      (return))))

(fn CancelReading
  (bind _wp_basehud (Variables|Default|GetWP_BaseHUD))
  (Class|Image|SetBrush (Variables|/Game/Dynamic/Blueprints/Prototype/UserInterface/HUD/WP_BaseHUD.WP_BaseHUD_C|GetReadingImage _wp_basehud) (Utilities|Struct|MakeSlateBrush "NoDrawType" "NoTile" "NoMirror" "(X=700.000000,Y=900.000000)" "(Left=0.000000,Top=0.000000,Right=0.000000,Bottom=0.000000)" "(SpecifiedColor=(R=1.000000,G=1.000000,B=1.000000,A=1.000000),ColorUseRule=UseColor_Specified)" "(CornerRadii=(X=0.000000,Y=0.000000,Z=0.000000,W=1.000000),Color=(SpecifiedColor=(R=0.000000,G=0.000000,B=0.000000,A=0.000000),ColorUseRule=UseColor_Specified),Width=0.000000,RoundingType=HalfHeightRadius,bUseBrushTransparency=False)" 0))
  (Class|BackgroundBlur|SetBlurStrength (Variables|/Game/Dynamic/Blueprints/Prototype/UserInterface/HUD/WP_BaseHUD.WP_BaseHUD_C|GetBackgroundBlur _wp_basehud) 0.0)
  (Variables|/Script/TheSeventhProof.PlayerCharacter|SetPlayerStates (Variables|Default|GetBP_BasePlayer) "EPS_Normal"))

(fn InteractInspectables
  (CallFunction|SelectCrosshair 0 "(X=5.000000,Y=5.000000)" 0.0))

(fn CancelInspecting
  (Variables|/Script/Engine.CharacterMovementComponent|SetMaxWalkSpeed (Variables|/Script/Engine.Character|GetCharacterMovement (Variables|Default|GetBP_BasePlayer)) 2e+02))